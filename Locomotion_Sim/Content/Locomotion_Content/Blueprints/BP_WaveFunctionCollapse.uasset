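; Seeded tile-map generator that builds a grid of wall modules with scattered balls and exports it to JSON.
; The construction script forces wall and corner pieces on borders, randomizes interior modules and rotations, and renders them as instanced static meshes.
; BeginPlay spawns the stored balls and saves cells, balls and seed to the project's Python folder.
; Despite the WaveFunctionCollapse name, interior placement applies no adjacency constraints.
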(event EventBeginPlay
  (bind _randomstream (Variables|Random|GetRandomStream))
  (Math|Random|SetRandomStreamSeed _randomstream (Variables|Random|GetRandomStreamSeed))
  (Class|KismetMathLibrary|SeedRandomStream _randomstream)
  (CallFunction|StartMapGeneration)
  (CallFunction|SerializeandOutputGrid))

(fn ConstructionScript
  (bind _moduletemplates (Variables|Default|GetModuleTemplates))
  (bind _materialarray (Variables|ForTheBalls|GetMaterialArray))
  (bind _storedtransforms (Variables|ForTheBalls|GetStoredTransforms))
  (bind _defaultsceneroot (Variables|Default|GetDefaultSceneRoot))
  (bind _randomstream (Variables|Random|GetRandomStream))
  (bind _wfc_cell_row (Variables|Default|GetWFC_Cell_Row))
  (bind _cell_row (Utilities|Struct|BreakWFC_Cell_Grid_Row _wfc_cell_row))
  (bind _uniquetransform (CallFunction|GetRandomUniqueTransform _storedtransforms))
  (bind _returnvalue (Transformation|GetRelativeTransform _defaultsceneroot))
  (bind (_gridindices _transform) (Utilities|Struct|BreakIndicesAndTransforms _uniquetransform))
  (bind (_location _rotation _scale) (Math|Transform|BreakTransform _returnvalue))
  (CallFunction|SetInstancedStaticMeshes)
  (for _index (range 0 (- (Variables|Default|GetMapYLen) 1))
    (for _index_2 (range 0 (- (Variables|Default|GetMapYLen) 1))
      (if (.IsOnBorder (CallFunction|IsonBorder _index _index_2 (Variables|Default|GetMapXLen) (Variables|Default|GetMapYLen)))
        (Variables|RotationIndices|SetCurrRotationIndex (.RotationIndex (CallFunction|IsonBorder _index _index_2 (Variables|Default|GetMapXLen) (Variables|Default|GetMapYLen))))
        (Variables|Random|SetCurrentRandomModuleIndex (.ModuleIndex (CallFunction|IsonBorder _index _index_2 (Variables|Default|GetMapXLen) (Variables|Default|GetMapYLen))))
        (else
          (bind _output_get (Variables|RotationIndices|SetCurrRotationIndex (Class|KismetMathLibrary|RandomIntegerfromStream _randomstream 4)))
          (bind _output_get_2 (Variables|Random|SetCurrentRandomModuleIndex (Class|KismetMathLibrary|RandomIntegerfromStream _randomstream (Utilities|Array|Length _moduletemplates))))))
      (if (== (Utilities|Array|Get(acopy) _moduletemplates _output_get_2) "/Game/Locomotion_Content/Blueprints/Modules/BP_WFC_Mod_No_walls.BP_WFC_Mod_No_walls_C")
        (Variables|RotationIndices|SetCurrRotationIndex 0))
      (bind _structout (Utilities|Struct|SetmembersinWFC_Cell (Variables|Default|GetWFC_Cell) (CallFunction|VectortoGridPos (Variables|Default|GetDefault_X_Y_Offset) _index _index_2) (Utilities|Array|Get(acopy) _moduletemplates _output_get_2) _output_get _output_get_2 (Math|Vector2D|MakeVector2D (Math|Conversions|ToFloat(Integer) _index_2) (Math|Conversions|ToFloat(Integer) _index))))
      (bind _output_get_3 (Variables|Default|SetWFC_Cell _structout))
      (Utilities|Array|Add _cell_row _output_get_3)
      (bind _structout_2 (Utilities|Struct|SetmembersinIndicesAndTransforms (Variables|ForTheBalls|GetCurrentTransform) (Math|Vector2D|MakeVector2D (Math|Conversions|ToFloat(Integer) _index_2) (Math|Conversions|ToFloat(Integer) _index)) (Math|Transform|MakeTransform (+ (Math|Vector|MakeVector (.X (Math|Vector2D|BreakVector2D (CallFunction|VectortoGridPos (Variables|Default|GetDefault_X_Y_Offset) _index _index_2))) (.Y (Math|Vector2D|BreakVector2D (CallFunction|VectortoGridPos (Variables|Default|GetDefault_X_Y_Offset) _index _index_2))) 0.0) _location) _rotation _scale)))
      (Utilities|Array|Add (Variables|ForTheBalls|GetStoredTransforms) _structout_2)
      (Components|InstancedStaticMesh|AddInstance (.Current_ISMC (CallFunction|MakeInstanceTransform (Utilities|Array|Get(acopy) _moduletemplates _output_get_2) (Math|Transform|MakeTransform (+ (Math|Vector|MakeVector (.X (Math|Vector2D|BreakVector2D (CallFunction|VectortoGridPos (Variables|Default|GetDefault_X_Y_Offset) _index _index_2))) (.Y (Math|Vector2D|BreakVector2D (CallFunction|VectortoGridPos (Variables|Default|GetDefault_X_Y_Offset) _index _index_2))) 0.0) _location) _rotation _scale) _output_get)) (.NewTransform (CallFunction|MakeInstanceTransform (Utilities|Array|Get(acopy) _moduletemplates _output_get_2) (Math|Transform|MakeTransform (+ (Math|Vector|MakeVector (.X (Math|Vector2D|BreakVector2D (CallFunction|VectortoGridPos (Variables|Default|GetDefault_X_Y_Offset) _index _index_2))) (.Y (Math|Vector2D|BreakVector2D (CallFunction|VectortoGridPos (Variables|Default|GetDefault_X_Y_Offset) _index _index_2))) 0.0) _location) _rotation _scale) _output_get)) true))
    (Utilities|Array|Add (Variables|Default|GetWFC_Grid) (Variables|Default|GetWFC_Cell_Row))
    (Utilities|Array|Clear _cell_row))
  (Rendering|Material|SetScalarParameterValue "/Game/Locomotion_Content/Blueprints/HeightOpacityMasking.HeightOpacityMasking" "MapHeight" (.Z (Math|Vector|BreakVector (.Location (Math|Transform|BreakTransform (Transformation|GetWorldTransform (Variables|Default|GetDefaultSceneRoot)))))) :!class /Script/Engine.KismetMaterialLibrary)
  (Rendering|Material|SetScalarParameterValue "/Game/Locomotion_Content/Blueprints/HeightOpacityMasking.HeightOpacityMasking" "RoofOffset" 1e+02 :!class /Script/Engine.KismetMaterialLibrary)
  (for _index_3 (range 0 (Variables|Default|GetMaxBalls))
    (bind _output_get_4 (Variables|ForTheBalls|SetMaterialIndex (Class|KismetMathLibrary|RandomIntegerfromStream (Variables|Random|GetRandomStream) (Utilities|Array|Length _materialarray))))
    (bind _structout_3 (Utilities|Struct|SetmembersinWFC_Sphere (Variables|Default|GetWFC_Sphere) _gridindices (Utilities|Array|Get(acopy) _materialarray _output_get_4) _output_get_4 _transform))
    (Utilities|Array|Add (Variables|Default|GetSpheresToRender) _structout_3)))

(fn CreateBaseModuleInstances
  (for (_array_element _array_index) (Variables|Default|GetModuleTemplates)
    (bind _returnvalue (Game|SpawnActorfromClass _array_element (Transformation|GetActorTransform) "Undefined" "MultiplyWithRoot" 0 0 0))))

(fn GetValidSockets
  (params (SocketType :type E_WFC_Socket_Name%20Enum :default "NewEnumerator0") (MapGrid :type Array%20of%20Booleans))
  (switch string (Utilities|String|EnumtoString SocketType)
    (:No_Walls_S
      _)
    (:Corner_Wall_0
      (return (Variables|SocketRules|GetCorner_Wall_0_Cons)))
    (:Corner_Wall_1
      (return (Variables|SocketRules|GetCorner_Wall_1_Cons)))
    (:Hall_0
      _)
    (:Side_Wall_0
      (return (Variables|SocketRules|GetSide_Wall_0)))
    (:Side_Wall_1
      (return (Variables|SocketRules|GetSide_Wall_1)))
    (:Side_Wall_2
      (return (Variables|SocketRules|GetSide_Wall_2)))
    (:Nothing
      (return (Variables|SocketRules|GetNothing))))
  (return (Variables|SocketRules|GetNo_Walls_Cons)))

(fn StartMapGeneration
  (for _array_element (Variables|Default|GetSpheresToRender)
    (Game|SpawnActorfromClass "/Game/Locomotion_Content/Blueprints/BP_WFC_Ball_Master.BP_WFC_Ball_Master_C" (.Transform (Utilities|Struct|BreakWFC_Sphere _array_element)) "Undefined" "MultiplyWithRoot" 0 (.MaterialIndex (Utilities|Struct|BreakWFC_Sphere _array_element)) 0)))

(fn Vector2DtoTransform
  (params (XYPos :type Vector%202D%20Structure))
  (bind _returnvalue (Transformation|GetActorTransform))
  (bind (_x _y) (Math|Vector2D|BreakVector2D XYPos))
  (bind _default_x_y_offset (Variables|Default|GetDefault_X_Y_Offset))
  (bind (_x_2 _y_2) (Math|Vector2D|BreakVector2D _default_x_y_offset))
  (bind (_location _rotation _scale) (Math|Transform|BreakTransform _returnvalue))
  (return (Math|Transform|MakeTransform (Math|Vector|MakeVector (- _x _x_2) (- _y _y_2) (.Z (Math|Vector|BreakVector _location))) _rotation _scale)))

(fn VectortoGridPos
  (params (InputVector2D :type Vector%202D%20Structure) (RowIndex :type Integer) (ColumnIndex :type Integer))
  (bind (_x _y) (Math|Vector2D|BreakVector2D InputVector2D))
  (bind _gridposoffset (LocalVariables|GetGridPosOffset))
  (return (Math|Vector2D|MakeVector2D (* _x (* ColumnIndex _gridposoffset)) (* _y (* RowIndex _gridposoffset)))))

(fn IsonBorder
  (params (RowIndex :type Integer) (ColumnIndex :type Integer) (GridRowLength :type Integer) (GridColumnLength :type Integer))
  (bind _sidewallindex (Variables|RotationIndices|GetSideWallIndex))
  (bind _cornerwallindex (Variables|RotationIndices|GetCornerWallIndex))
  (if (Math|Boolean|ANDBoolean (== RowIndex 0) (== ColumnIndex 0) (Variables|Default|GetOpenBLCorner))
    _
    (else
      ;[1 1 1] Bottom Border
      (if (Math|Boolean|ANDBoolean (>= RowIndex 0) (<= RowIndex (- GridRowLength 1)) (== ColumnIndex 0))
        ;[1 1 1] Bottom Left Corner
        (if (== RowIndex 0)
          (return true "/Game/Locomotion_Content/Blueprints/Modules/BP_WFC_Mod_Corner_Wall.BP_WFC_Mod_Corner_Wall_C" (Variables|RotationIndices|GetCornerWallBottomLeftIndex) _cornerwallindex)
          (else
            ;[1 1 1] Bottom Right Corner -> Bottom Border
            (if (== RowIndex (- GridRowLength 1))
              (return true "/Game/Locomotion_Content/Blueprints/Modules/BP_WFC_Mod_Corner_Wall.BP_WFC_Mod_Corner_Wall_C" (Variables|RotationIndices|GetCornerWallBottomRightIndex) _cornerwallindex)
              (else
                (return true "/Game/Locomotion_Content/Blueprints/Modules/BP_WFC_Mod_Side_Wall.BP_WFC_Mod_Side_Wall_C" (Variables|RotationIndices|GetSideWallBottomBorderRotationIndex) _sidewallindex)))))
        (else
          ;[1 1 1] Top Border
          (if (Math|Boolean|ANDBoolean (>= RowIndex 0) (<= RowIndex (- GridRowLength 1)) (== ColumnIndex (- GridColumnLength 1)))
            ;[1 1 1] Top Left Corner
            (if (== RowIndex 0)
              (return true "/Game/Locomotion_Content/Blueprints/Modules/BP_WFC_Mod_Corner_Wall.BP_WFC_Mod_Corner_Wall_C" (Variables|RotationIndices|GetCornerWallTopLeftIndex) _cornerwallindex)
              (else
                ;[1 1 1] Top Right Corner -> Top Border
                (if (== RowIndex (- GridRowLength 1))
                  (return true "/Game/Locomotion_Content/Blueprints/Modules/BP_WFC_Mod_Corner_Wall.BP_WFC_Mod_Corner_Wall_C" (Variables|RotationIndices|GetCornerWallTopRightIndex) _cornerwallindex)
                  (else
                    (return true "/Game/Locomotion_Content/Blueprints/Modules/BP_WFC_Mod_Side_Wall.BP_WFC_Mod_Side_Wall_C" (Variables|RotationIndices|GetSideWallTopBorderRotationIndex) _sidewallindex)))))
            (else
              ;[1 1 1] Left Border
              (if (Math|Boolean|ANDBoolean (>= ColumnIndex 0) (<= ColumnIndex (- GridColumnLength 1)) (== RowIndex 0))
                ;[1 1 1] Bottom Left Corner
                (if (== ColumnIndex 0)
                  (return true "/Game/Locomotion_Content/Blueprints/Modules/BP_WFC_Mod_Corner_Wall.BP_WFC_Mod_Corner_Wall_C" (Variables|RotationIndices|GetCornerWallBottomLeftIndex) _cornerwallindex)
                  (else
                    ;[1 1 1] Top Left Corner -> Left Border
                    (if (== ColumnIndex (- GridColumnLength 1))
                      (return true "/Game/Locomotion_Content/Blueprints/Modules/BP_WFC_Mod_Corner_Wall.BP_WFC_Mod_Corner_Wall_C" (Variables|RotationIndices|GetCornerWallTopLeftIndex) _cornerwallindex)
                      (else
                        _))))
                (else
                  ;[1 1 1] Right Border
                  (if (Math|Boolean|ANDBoolean (>= ColumnIndex 0) (<= ColumnIndex (- GridColumnLength 1)) (== RowIndex (- GridRowLength 1)))
                    ;[1 1 1] Top Right Corner
                    (if (== ColumnIndex (- GridColumnLength 1))
                      (return true "/Game/Locomotion_Content/Blueprints/Modules/BP_WFC_Mod_Corner_Wall.BP_WFC_Mod_Corner_Wall_C" (Variables|RotationIndices|GetCornerWallTopRightIndex) _cornerwallindex)
                      (else
                        ;[1 1 1] Bottom Right Corner -> Right Border
                        (if (== ColumnIndex 0)
                          (return true "/Game/Locomotion_Content/Blueprints/Modules/BP_WFC_Mod_Corner_Wall.BP_WFC_Mod_Corner_Wall_C" (Variables|RotationIndices|GetCornerWallBottomRightIndex) _cornerwallindex)
                          (else
                            (return true "/Game/Locomotion_Content/Blueprints/Modules/BP_WFC_Mod_Side_Wall.BP_WFC_Mod_Side_Wall_C" (Variables|RotationIndices|GetSideWallRightBorderRotationIndex) _sidewallindex)))))
                    (else
                      ;[1 1 1] Not On Border
                      (return false 0 0 0)))))))))))
  (return true "/Game/Locomotion_Content/Blueprints/Modules/BP_WFC_Mod_Side_Wall.BP_WFC_Mod_Side_Wall_C" (Variables|RotationIndices|GetSideWallLeftBorderRotationIndex) _sidewallindex))

(fn GetRandomUniqueTransform
  (params (ItemList :type Array%20of%20Indices%20and%20Transforms%20Structures))
  (bind _returnvalue (Utilities|Array|Length ItemList))
  (bind _chosenindices (Variables|Random|GetRandomUniqueItem|GetChosenIndices))
  (bind _randomstream (Variables|Random|GetRandomStream))
  (bind _returnvalue_2 (Class|KismetMathLibrary|RandomIntegerfromStream _randomstream _returnvalue))
  (if (== (Utilities|Array|Length _chosenindices) 0)
    (Utilities|Array|Add _chosenindices (Class|KismetMathLibrary|RandomIntegerfromStream _randomstream _returnvalue))
    (else
      (while (or (Variables|Random|GetRandomUniqueItem|GetFoundUniqueIndex) (> (Variables|Random|GetRandomUniqueItem|GetForceQuitLoop) _returnvalue))
        (Variables|Random|GetRandomUniqueItem|SetFoundUniqueIndex (not (Utilities|Array|ContainsItem _chosenindices _returnvalue_2)))
        (Variables|Random|GetRandomUniqueItem|SetForceQuitLoop (+ (Variables|Random|GetRandomUniqueItem|GetForceQuitLoop) 1)))
      (Utilities|Array|Add _chosenindices _returnvalue_2)
      (if (> (Variables|Random|GetRandomUniqueItem|GetForceQuitLoop) _returnvalue)
        (Development|PrintString "Exceeded Length of List"))
      (Variables|Random|GetRandomUniqueItem|SetForceQuitLoop 0)))
  (return (Utilities|Array|Get(acopy) ItemList _returnvalue_2)))

(fn SerializeandOutputGrid
  (for (_array_element _array_index) (Variables|Default|GetWFC_Grid)
    (for (_array_element_2 _array_index_2) (Utilities|Struct|BreakWFC_Cell_Grid_Row _array_element)
      (bind _outjsonstring (|StructtoJsonString _array_element_2))
      (Variables|Default|SetJSONString (Utilities|String|Append (Variables|Default|GetJSONString) "\"cell_row" (Utilities|String|ToString(Integer) _array_index) "_col" (Utilities|String|ToString(Integer) _array_index_2) "\": " _outjsonstring ","))))
  (for (_array_element_3 _array_index_3) (Variables|Default|GetSpheresToRender)
    (bind _outjsonstring_2 (|StructtoJsonString _array_element_3))
    (Variables|Default|SetJSONString (Utilities|String|Append (Variables|Default|GetJSONString) "\"sphere_" (Utilities|String|ToString(Integer) _array_index_3) "\": " _outjsonstring_2 ",")))
  (bind _outjsonstring_3 (|StructtoJsonString (Variables|Default|GetDefault_X_Y_Offset)))
  (bind _output_get (Variables|Default|SetJSONString (Utilities|String|Append (Variables|Default|GetJSONString) "\"offsets\": " _outjsonstring_3 ", \"rowLength\": " (Utilities|String|ToString(Integer) (Variables|Default|GetMapXLen)) " , \"columnLength\": " (Utilities|String|ToString(Integer) (Variables|Default|GetMapYLen)) ", \"mapSeed\": " (Utilities|String|ToString(Integer) (Variables|Random|GetRandomStreamSeed)) "}")))
  (Class|VictoryBPFunctionLibrary|FileIOSaveStringTexttoFile (Utilities|String|Append (.PathPart (Utilities|String|Split (Class|BlueprintPathsLibrary|GetProjectFilePath))) "/Python") "map_output.json" _output_get true false))

(fn SetInstancedStaticMeshes
  (bind _defaultsceneroot (Variables|Default|GetDefaultSceneRoot))
  (bind _returnvalue (Transformation|GetRelativeTransform _defaultsceneroot))
  (bind _returnvalue_2 (AddComponent|AddInstancedStaticMeshComponent false _returnvalue))
  (bind _output_get (Variables|ISMC|SetISMC_Side_Wall _returnvalue_2))
  (Components|StaticMesh|SetStaticMesh _output_get "/Game/Locomotion_Content/Modules/Meshes/Side_Wall.Side_Wall")
  (bind _returnvalue_3 (AddComponent|AddInstancedStaticMeshComponent false _returnvalue))
  (bind _output_get_2 (Variables|ISMC|SetISMC_Corner_Wall _returnvalue_3))
  (Components|StaticMesh|SetStaticMesh _output_get_2 "/Game/Locomotion_Content/Modules/Meshes/Corner_Wall.Corner_Wall")
  (bind _returnvalue_4 (AddComponent|AddInstancedStaticMeshComponent false _returnvalue))
  (bind _output_get_3 (Variables|ISMC|SetISMC_No_Walls _returnvalue_4))
  (Components|StaticMesh|SetStaticMesh _output_get_3 "/Game/Locomotion_Content/Modules/Meshes/No_Walls.No_Walls"))

(fn MakeInstanceTransform
  (params (Class :type BP%20WFC%20Module%20Master%20Class%20Reference) (OrgTransform :type Transform) (RotationIndex :type Integer))
  (bind (_location _rotation _scale) (Math|Transform|BreakTransform OrgTransform))
  (bind _returnvalue (+ RotationIndex 1))
  (bind _returnvalue_2 (Math|Integer|%(Integer) _returnvalue 4))
  (bind _returnvalue_3 (* _returnvalue_2 90))
  (bind _returnvalue_4 (Math|Conversions|ToFloat(Integer) _returnvalue_3))
  (bind _returnvalue_5 (Math|Rotator|MakeRotator 0.0 0.0 _returnvalue_4))
  (if (== Class "/Game/Locomotion_Content/Blueprints/Modules/BP_WFC_Mod_Corner_Wall.BP_WFC_Mod_Corner_Wall_C")
    (bind _output_get (Variables|ISMC|SetCurr_Offset (Variables|ISMC|GetCorner_Wall_Offsets)))
    (bind _newlocation (CallFunction|ApplyTransformOffsets RotationIndex _output_get _location))
    (bind _output_get_2 (Variables|ISMC|SetReturnTransform (Math|Transform|MakeTransform _newlocation _returnvalue_5 _scale)))
    (bind _output_get_3 (Variables|ISMC|SetCurrent_ISMC (Variables|ISMC|GetISMC_Corner_Wall)))
    (elif (== Class "/Game/Locomotion_Content/Blueprints/Modules/BP_WFC_Mod_No_walls.BP_WFC_Mod_No_walls_C")
      (Variables|ISMC|SetCurr_Offset (Variables|ISMC|GetNo_Walls_Offset))
      (bind _newlocation_2 (CallFunction|ApplyTransformOffsets RotationIndex _output_get _location))
      (Variables|ISMC|SetReturnTransform (Math|Transform|MakeTransform (+ _newlocation_2 (Math|Vector|MakeVector 0.0 0.0 (* (.Z (Math|Vector|BreakVector _output_get)) 2.0))) _returnvalue_5 _scale))
      (Variables|ISMC|SetCurrent_ISMC (Variables|ISMC|GetISMC_No_Walls))
      (else
        (Variables|ISMC|SetCurr_Offset (Variables|ISMC|GetSide_Wall_Offsets))
        (bind _newlocation_3 (CallFunction|ApplyTransformOffsets RotationIndex _output_get _location))
        (Variables|ISMC|SetReturnTransform (Math|Transform|MakeTransform _newlocation_3 _returnvalue_5 _scale))
        (Variables|ISMC|SetCurrent_ISMC (Variables|ISMC|GetISMC_Side_Wall)))))
  (return _output_get_2 _output_get_3))

(fn ApplyTransformOffsets
  (params (RotationIndex :type Integer) (CurrOffsets :type Vector) (OrgLocation :type Vector))
  (bind (_x _y) (Math|Vector|BreakVector CurrOffsets))
  (if (== RotationIndex 0)
    (return (+ OrgLocation (Math|Vector|MakeVector (* (.X (Math|Vector|BreakVector CurrOffsets)) -2.0) 0.0 0.0)))
    (elif (== RotationIndex 1)
      (return (- OrgLocation (Math|Vector|MakeVector (* _x 2.0) (* _y 2.0) 0.0)))
      (elif (== RotationIndex 2)
        (return (- OrgLocation (Math|Vector|MakeVector 0.0 (* (.Y (Math|Vector|BreakVector CurrOffsets)) 2.0) 0.0)))
        (else
          (return OrgLocation))))))