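; Master module for Wave Function Collapse (WFC) tiles, holding an enum socket on each X and Y side and showing them as text labels.
; Construction caches the starting sockets and builds a name-to-enum map.
; RotateModule applies a local rotation, cycles sockets between sides by RotationIndex and refreshes labels.
; RotateSocket encodes orientation in enum names, remapping numeric suffixes modulo 4 and leaving "S" sockets unchanged.
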(event Custom|RotateModule
  (bind _rotationindex (Variables|WFC|GetRotationIndex))
  (bind _startsockets (Variables|Default|GetStartSockets))
  (bind _rotationindex_2 (Variables|WFC|GetRotationIndex))
  (Transformation|AddLocalRotation (Variables|Default|GetDefaultSceneRoot) (Math|Rotator|MakeRotfromZ (Math|Vector|MakeVector 0.0 0.0 (Math|Conversions|ToFloat(Integer) (* _rotationindex 90)))) false false)
  (Variables|WFC|Sockets|SetPosXSocket (CallFunction|RotateSocket (Utilities|Array|Get(acopy) _startsockets (Math|Integer|%(Integer) _rotationindex 4)) _rotationindex_2))
  (Variables|WFC|Sockets|SetNegYSocket (CallFunction|RotateSocket (Utilities|Array|Get(acopy) _startsockets (Math|Integer|%(Integer) (+ _rotationindex 3) 4)) _rotationindex_2))
  (Variables|WFC|Sockets|SetNegXSocket (CallFunction|RotateSocket (Utilities|Array|Get(acopy) _startsockets (Math|Integer|%(Integer) (+ _rotationindex 2) 4)) _rotationindex_2))
  (Variables|WFC|Sockets|SetPosYSocket (CallFunction|RotateSocket (Utilities|Array|Get(acopy) _startsockets (Math|Integer|%(Integer) (+ _rotationindex 1) 4)) _rotationindex_2))
  (CallFunction|UpdateDisplayText))

(fn ConstructionScript
  (Utilities|Map|Clear (Variables|WFC|Sockets|GetSocketMap))
  (bind _enumvalue (|ForEachE_WFC_Socket_Name)
    (:LoopBody
      (Utilities|Map|Add (Variables|WFC|Sockets|GetSocketMap) (Utilities|String|EnumtoString _enumvalue) _enumvalue))
    (:then
      (Variables|Default|SetStartSockets (Utilities|Array|MakeArray (Variables|WFC|Sockets|GetPosXSocket) (Variables|WFC|Sockets|GetPosYSocket) (Variables|WFC|Sockets|GetNegXSocket) (Variables|WFC|Sockets|GetNegYSocket)))
      (CallFunction|UpdateDisplayText))))

(fn UpdateDisplayText
  (Rendering|Components|TextRender|SetText (Variables|Default|GetPosX) (Utilities|Text|ToText(String) (Utilities|String|EnumtoString (Variables|WFC|Sockets|GetPosXSocket))))
  (Rendering|Components|TextRender|SetText (Variables|Default|GetNegX) (Utilities|Text|ToText(String) (Utilities|String|EnumtoString (Variables|WFC|Sockets|GetNegXSocket))))
  (Rendering|Components|TextRender|SetText (Variables|Default|GetPosY) (Utilities|Text|ToText(String) (Utilities|String|EnumtoString (Variables|WFC|Sockets|GetPosYSocket))))
  (Rendering|Components|TextRender|SetText (Variables|Default|GetNegY) (Utilities|Text|ToText(String) (Utilities|String|EnumtoString (Variables|WFC|Sockets|GetNegYSocket)))))

(fn RotateSocket
  (params (InSocket :type E_WFC_Socket_Name%20Enum :default "NewEnumerator0") (RotationIndex :type Integer))
  (bind _returnvalue (Utilities|String|EnumtoString InSocket))
  (bind _returnvalue_2 (Utilities|String|ParseIntoArray _returnvalue "_"))
  (bind _returnvalue_3 (Utilities|Array|Length _returnvalue_2))
  (bind _returnvalue_4 (- _returnvalue_3 1))
  (bind _output (Utilities|Array|Get(acopy) _returnvalue_2 _returnvalue_4))
  (switch string _output
    (:Default
      (return (.Value (Utilities|Map|Find (Variables|WFC|Sockets|GetSocketMap) (Utilities|String|Append (Utilities|String|GetSubstring _returnvalue 0 _returnvalue_4) (Utilities|String|ToString(Integer) (Math|Integer|%(Integer) (+ (Math|Conversions|ToInteger(Byte) _output) RotationIndex) 4)))))))
    (:S
      (return InSocket))))